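; Player controller for LeaveMeAlone that opens the pause, game over and death screens.
; Pressing Pause, if not already paused, stops the pawn's weapon fire, pauses the game and shows the pause widget.
; EndTimeGame shows game over unless the player is dead, while OnDead flags death and shows the death widget after a short delay.
; Each screen switches input to UI-only and shows the cursor.
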(event `InputAction|Pause`
  (params (Key :type "Key Structure"))
  (bind _returnvalue (`self.K2_GetPawn` self))
  (:`Pressed`
    (if (not (`self.OnPause`))
      (set `self.OnPause` true)
      (`/Engine/EditorBlueprintResources/StandardMacros.IsValid` _returnvalue
        (:`Is Valid`
          (`LMAWeaponComponent.FireStop` (`self.GetComponentByClass` _returnvalue "/Script/LeaveMeAlone.LMAWeaponComponent")))
        (:`Is Not Valid`
          _))
      (`GameplayStatics.SetGamePaused` true)
      (bind _returnvalue_2 (`|CreateWidget` "/Game/LeaveMeAlone/Widgets/UI/WBP_Pause.WBP_Pause_C"))
      (bind _output_get (set `self.Pause Widget` _returnvalue_2))
      (`UserWidget.AddToViewport` _output_get 0)
      (`WidgetBlueprintLibrary.SetInputMode_UIOnlyEx` self _output_get)
      (set `self.bShowMouseCursor` true))))

(event `EndTimeGame`
  (if (not (`self.IsDead`))
    (bind _returnvalue (`|CreateWidget` "/Game/LeaveMeAlone/Widgets/UI/WBP_GameOver.WBP_GameOver_C"))
    (bind _output_get (set `self.GameOver` _returnvalue))
    (`UserWidget.AddToViewport` _output_get 0)
    (`WidgetBlueprintLibrary.SetInputMode_UIOnlyEx` self _output_get)
    (set `self.bShowMouseCursor` true)))

(event `OnDead`
  (set `self.IsDead` true)
  (`KismetSystemLibrary.Delay` 3.0)
  (bind _returnvalue (`|CreateWidget` "/Game/LeaveMeAlone/Widgets/UI/WBP_Dead.WBP_Dead_C"))
  (bind _output_get (set `self.Dead` _returnvalue))
  (`UserWidget.AddToViewport` _output_get 0)
  (`WidgetBlueprintLibrary.SetInputMode_UIOnlyEx` self _output_get)
  (set `self.bShowMouseCursor` true))

(fn `UserConstructionScript`)